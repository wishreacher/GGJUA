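; Player Blueprint for a strategy game where mana and water, replenished by a timer, pay for trees, units and an Ent attack.
; Input keys toggle placement and targeting modes, with Tick moving a unit preview or cursor effect.
; Left click traces under the mouse to place, attack or activate resource spots.
; Placement spawns the actor first to read its cost, destroying it if unaffordable; the radial-damage Ent attack has a cooldown.
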(event Custom|Add%20Resources
  (Variables|Resources|SetCurrentMana (+ (Variables|Resources|GetCurrentMana) (Variables|Resources|GetManaIncomeRate)))
  (Variables|Resources|SetCurrentWater (+ (Variables|Resources|GetCurrentWater) (Variables|Resources|GetWaterIncomeRate))))

(event EventBeginPlay
  (Variables|Resources|SetCurrentMana (Variables|Resources|GetMaxMana))
  (Variables|Resources|SetCurrentWater (Variables|Resources|GetMaxWater))
  (Utilities|Time|SetTimerbyEvent (delegate Custom|Add%20Resources) 0.5 true)
  (Utilities|FlowControl|Delay 0.2)
  (Actor|Tick|SetActorTickEnabled true))

(event EventTick
  (params (DeltaSeconds :type Float%20%28single-precision%29))
  (CallFunction|HandleRepresentationUnit)
  (CallFunction|HandleEntAttackRepresentation))

(event Input|ActionEvents|InputActionUnit1
  (params (Key :type Key%20Structure))
  (:Pressed
    (if (Variables|Default|GetShouldTraceForUnitPlacement)
      (CallFunction|DisableUnitPlacement)
      (else
        (CallFunction|AttempttoSpawnUnit "/Game/Blueprints/Allies/Hammer/BP_Hammer.BP_Hammer_C")
        (CallFunction|DisableTreePlacement)))))

(event Input|ActionEvents|InputActionUnit2
  (params (Key :type Key%20Structure))
  (:Pressed
    (if (Variables|Default|GetShouldTraceForUnitPlacement)
      (CallFunction|DisableUnitPlacement)
      (else
        (CallFunction|AttempttoSpawnUnit "/Game/Blueprints/Allies/Wizard/BP_Wizard.BP_Wizard_C")
        (CallFunction|DisableTreePlacement)))))

(event Input|ActionEvents|InputActionUnit3
  (params (Key :type Key%20Structure)))

(event Input|ActionEvents|InputActionTree1
  (params (Key :type Key%20Structure))
  (:Pressed
    (if (Variables|Default|GetbShouldTraceForTreePlaces)
      (CallFunction|DisableTreePlacement)
      (else
        (CallFunction|AttempttoSpawnTree "/Game/Blueprints/Towers/BP_SingleShotTree.BP_SingleShotTree_C")
        (CallFunction|DisableUnitPlacement)))))

(event Input|ActionEvents|InputActionTree2
  (params (Key :type Key%20Structure))
  (:Pressed
    (if (Variables|Default|GetbShouldTraceForTreePlaces)
      (CallFunction|DisableTreePlacement)
      (else
        (CallFunction|AttempttoSpawnTree "/Game/Blueprints/Towers/BP_AoEShotTree.BP_AoEShotTree_C")
        (CallFunction|DisableUnitPlacement)))))

(event Input|ActionEvents|InputActionEntAttack
  (params (Key :type Key%20Structure))
  (:Pressed
    (if (Variables|Default|GetCanUseEntAttack)
      (Utilities|FlowControl|FlipFlop
        (:A
          (Variables|Default|SetShouldTraceForEntAttack true)
          (CallFunction|DisableTreePlacement)
          (CallFunction|DisableUnitPlacement))
        (:B
          (Variables|Default|SetShouldTraceForEntAttack false))))))

(event Input|MouseEvents|LeftMouseButton
  (params (Key :type Key%20Structure))
  (bind _returnvalue (Game|GetPlayerController 0))
  (bind (_worldlocation _worlddirection) (Game|Player|ConvertMouseLocationToWorldSpace _returnvalue))
  (:Pressed
    (|TreePlacement)
    (|UnitPlacement)
    (|Entattack)
    (bind _outhit (Collision|LineTraceByChannel _worldlocation (+ _worldlocation (* _worlddirection 5e+03)) "TraceTypeQuery1" false 0 "None"))
    (bind _asbp_resource_place (Utilities|Casting|CastToBP_ResourcePlace (.hitactor _outhit)))
    (Default|ActivateSpot _asbp_resource_place)))

(fn ConstructionScript)

(fn AttempttoSpawnTree
  (params (TreeClass :type BP%20Base%20Tree%20Class%20Reference))
  (CallFunction|HighlightAllAvailableTreePlaces)
  (Variables|Default|SetbShouldTraceForTreePlaces true)
  (Variables|Default|SetTowerClass TreeClass))

(fn HighlightAllAvailableTreePlaces
  (bind _outactors (Actor|GetAllActorsOfClass "/Game/Blueprints/Towers/BP_BaseTree.BP_BaseTree_C"))
  (for _array_element _outactors
    (if (not (Variables|/Script/GGJUA.BaseTower|GetbIsBuilt _array_element))
      (Rendering|SetVisibility (Variables|/Game/Blueprints/Towers/BP_BaseTree.BP_BaseTree_C|GetSpotLight _array_element) true false))))

(fn DisableTreePlacement
  (bind _outactors (Actor|GetAllActorsOfClass "/Game/Blueprints/Towers/BP_BaseTree.BP_BaseTree_C"))
  (for _array_element _outactors
    (Rendering|SetVisibility (Variables|/Game/Blueprints/Towers/BP_BaseTree.BP_BaseTree_C|GetSpotLight _array_element) false false))
  (Variables|Default|SetbShouldTraceForTreePlaces false))

(fn IsEnoughResourcesforTree
  (params (Tree :type Base%20Tower%20Object%20Reference))
  (return (and (>= (Variables|Resources|GetCurrentWater) (Variables|/Script/GGJUA.BaseTower|GetCostInWater Tree)) (>= (Variables|Resources|GetCurrentMana) (Variables|/Script/GGJUA.BaseTower|GetCostInMana Tree)))))

(fn ReduceResourcesbyTreeCost
  (params (Tree :type Base%20Tower%20Object%20Reference))
  (Variables|Resources|SetCurrentWater (- (Variables|Resources|GetCurrentWater) (Variables|/Script/GGJUA.BaseTower|GetCostInWater Tree)))
  (Variables|Resources|SetCurrentMana (- (Variables|Resources|GetCurrentMana) (Variables|/Script/GGJUA.BaseTower|GetCostInMana Tree))))

(fn AttempttoSpawnUnit
  (params (Unit%20Class :type Tree%20Unit%20Class%20Reference))
  (Variables|Default|SetShouldTraceForUnitPlacement true)
  (Variables|Default|SetTreeUnitClass Unit%20Class))

(fn DisableUnitPlacement
  (Variables|Default|SetShouldTraceForUnitPlacement false)
  (Variables|Default|SetTreeUnitClass 0))

(fn HandleRepresentationUnit
  (bind _returnvalue (Game|GetPlayerController 0))
  (bind (_worldlocation _worlddirection) (Game|Player|ConvertMouseLocationToWorldSpace _returnvalue))
  (if (Variables|Default|GetShouldTraceForUnitPlacement)
    (bind _outhit (Collision|LineTraceByChannel _worldlocation (+ _worldlocation (* _worlddirection 5e+03)) "TraceTypeQuery1" false 0 "None"))
    (Utilities|IsValid (Variables|Default|GetRepresentationActor)
      (:Is%20Valid
        (Transformation|SetActorLocation (Variables|Default|GetRepresentationActor) (Math|Vector|MakeVector (.x (.impactpoint _outhit)) (.y (.impactpoint _outhit)) (+ (.z (.impactpoint _outhit)) (Components|Capsule|GetScaledCapsuleHalfHeight (Variables|/Script/Engine.Character|GetCapsuleComponent (Variables|Default|GetRepresentationActor))))) false false))
      (:Is%20Not%20Valid
        (bind _returnvalue_2 (Game|SpawnActorfromClass (Variables|Default|GetTreeUnitClass) (Math|Transform|MakeTransform (Math|Vector|MakeVector (.x (.impactpoint _outhit)) (.y (.impactpoint _outhit)) (.z (.impactpoint _outhit)))) "AdjustIfPossibleButAlwaysSpawn" 0 0))
        (bind _output_get (Variables|Default|SetRepresentationActor _returnvalue_2))
        (Collision|SetActorEnableCollision _output_get false)))
    (else
      (Utilities|IsValid (Variables|Default|GetRepresentationActor)
        (:Is%20Valid
          (Actor|DestroyActor (Variables|Default|GetRepresentationActor)))))))

(fn IsEnoughResourcesforUnit
  (params (Tree :type Base%20Unit%20Object%20Reference))
  (return (and (<= (Variables|/Script/GGJUA.BaseUnit|GetManaCost Tree) (Variables|Resources|GetCurrentMana)) (<= (Variables|/Script/GGJUA.BaseUnit|GetWaterCost Tree) (Variables|Resources|GetCurrentWater)))))

(fn ReduceResourcesbyUnitCost
  (params (Unit :type Base%20Unit%20Object%20Reference))
  (Variables|Resources|SetCurrentMana (- (Variables|Resources|GetCurrentMana) (Variables|/Script/GGJUA.BaseUnit|GetManaCost Unit)))
  (Variables|Resources|SetCurrentWater (- (Variables|Resources|GetCurrentWater) (Variables|/Script/GGJUA.BaseUnit|GetWaterCost Unit))))

(fn HandleEntAttackRepresentation
  (bind _returnvalue (Game|GetPlayerController 0))
  (bind (_worldlocation _worlddirection) (Game|Player|ConvertMouseLocationToWorldSpace _returnvalue))
  (if (Variables|Default|GetShouldTraceForEntAttack)
    (bind _outhit (Collision|LineTraceByChannel _worldlocation (+ _worldlocation (* _worlddirection 5e+03)) "TraceTypeQuery1" false 0 "None"))
    (Utilities|IsValid (Variables|Default|GetEntPlacement)
      (:Is%20Valid
        (Transformation|SetWorldLocation (Variables|Default|GetEntPlacement) (.impactpoint _outhit) false false))
      (:Is%20Not%20Valid
        (bind _returnvalue_2 (Niagara|SpawnSystematLocation "/Game/UI/Cursor/FX_Cursor.FX_Cursor" (.impactpoint _outhit)))
        (Variables|Default|SetEntPlacement _returnvalue_2)))
    (else
      (Utilities|IsValid (Variables|Default|GetEntPlacement)
        (:Is%20Valid
          (Components|DestroyComponent (Variables|Default|GetEntPlacement)))))))

(event Custom|RechargeEntAttack
  (Variables|Default|SetCanUseEntAttack true)
  (Utilities|Time|ClearandInvalidateTimerbyHandle (Variables|Default|GetEntAbilityTimer))
  (Audio|PlaySound2D "/Game/SFX/ability_recovery.ability_recovery" 1.0 1.0 0.0 0 0))