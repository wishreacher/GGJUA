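; Player controller for a top-down style camera, with a visible, viewport-locked cursor, input-driven panning and stepped zoom.
; Input actions build a movement vector and a clamped zoom alpha, which MoveCamera applies to the player pawn every tick.
; Zoom alpha interpolates pan speed, pawn pitch and BP_Player spring arm length.
; Panning is not scaled by delta time, and the fetched mouse position is unused.
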(event EventBeginPlay
  (Input|SetInputModeGameandUI self 0 "LockAlways" true false)
  (Variables|Default|SetbShowMouseCursor true))

(event EventTick
  (params (DeltaSeconds :type Float%20%28single-precision%29))
  (CallFunction|MoveCamera))

(event Input|ActionEvents|InputActionMoveCameraLeft
  (params (Key :type Key%20Structure :default "None"))
  (:Pressed
    (Variables|Default|SetCameraMovement (- (Variables|Default|GetCameraMovement) "1.000000,0.000000,0.000000")))
  (:Released
    (Variables|Default|SetCameraMovement (+ (Variables|Default|GetCameraMovement) "1.000000,0.000000,0.000000"))))

(event Input|ActionEvents|InputActionMoveCameraUp
  (params (Key :type Key%20Structure :default "None"))
  (:Pressed
    (Variables|Default|SetCameraMovement (- (Variables|Default|GetCameraMovement) "0.000000,1.000000,0.000000")))
  (:Released
    (Variables|Default|SetCameraMovement (+ (Variables|Default|GetCameraMovement) "0.000000,1.000000,0.000000"))))

(event Input|ActionEvents|InputActionMoveCameraDown
  (params (Key :type Key%20Structure :default "None"))
  (:Pressed
    (Variables|Default|SetCameraMovement (+ (Variables|Default|GetCameraMovement) "0.000000,1.000000,0.000000")))
  (:Released
    (Variables|Default|SetCameraMovement (- (Variables|Default|GetCameraMovement) "0.000000,1.000000,0.000000"))))

(event Input|ActionEvents|InputActionMoveCameraRight
  (params (Key :type Key%20Structure :default "None"))
  (:Pressed
    (Variables|Default|SetCameraMovement (+ (Variables|Default|GetCameraMovement) "1.000000,0.000000,0.000000")))
  (:Released
    (Variables|Default|SetCameraMovement (- (Variables|Default|GetCameraMovement) "1.000000,0.000000,0.000000"))))

(event Input|ActionEvents|InputActionZoomIn
  (params (Key :type Key%20Structure :default "None"))
  (:Pressed
    (Variables|Default|SetCameraZoom (Math|Float|Clamp(Float) (- (Variables|Default|GetCameraZoom) 0.1)))))

(event Input|ActionEvents|InputActionZoomOut
  (params (Key :type Key%20Structure :default "None"))
  (:Pressed
    (Variables|Default|SetCameraZoom (Math|Float|Clamp(Float) (+ (Variables|Default|GetCameraZoom) 0.1)))))

(fn ConstructionScript)

(fn MoveCamera
  (bind _returnvalue (Game|Player|GetPlayerPawn 0))
  (bind _cameramovement (Variables|Default|GetCameraMovement))
  (bind _mincameraspeed (Variables|Default|GetMinCameraSpeed))
  (bind _maxcameraspeed (Variables|Default|GetMaxCameraSpeed))
  (bind _camerazoom (Variables|Default|GetCameraZoom))
  (bind _returnvalue_2 (Math|Vector|Normalize _cameramovement))
  (bind _returnvalue_3 (Math|Float|Lerp _mincameraspeed _maxcameraspeed _camerazoom))
  (bind _returnvalue_4 (Transformation|GetActorLocation _returnvalue))
  (bind _returnvalue_5 (* _returnvalue_2 _returnvalue_3))
  (bind _returnvalue_6 (+ (Math|Vector|MakeVector (.x _returnvalue_4) (.y _returnvalue_4) (.z _returnvalue_4)) _returnvalue_5))
  (bind _returnvalue_7 (Class|WidgetLayoutLibrary|GetMousePositiononViewport))
  (Variables|Default|SetMouseX (.x _returnvalue_7))
  (Variables|Default|SetMouseY (.y _returnvalue_7))
  (Transformation|SetActorLocationAndRotation _returnvalue (Math|Vector|MakeVector (.x _returnvalue_6) (.y _returnvalue_6) (.z _returnvalue_4)) (Math|Rotator|MakeRotator 0.0 (Math|Float|Lerp 15.0 0.0 (Variables|Default|GetCameraZoom)) -9e+01))
  (bind _asbp_player (Utilities|Casting|CastToBP_Player (Game|Player|GetPlayerPawn 0)))
  (Variables|/Script/Engine.SpringArmComponent|SetTargetArmLength (Variables|/Game/Blueprints/Player/BP_Player.BP_Player_C|GetSpringArm _asbp_player) (Math|Float|Lerp (Variables|Default|GetMinZoomDistance) (Variables|Default|GetMaxZoomDistance) (Variables|Default|GetCameraZoom))))