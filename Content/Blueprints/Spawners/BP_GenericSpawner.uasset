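; BP_GenericSpawner is a data-driven timed spawner that spawns actors at its own transform and registers them as the player's enemies.
; BeginPlay copies each DataTable row's class, spawn time and wave into parallel arrays.
; Tick spawns the current entry once game time reaches its timestamp, using a resettable DoOnce.
; It then advances the index and sets BP_Player's Wave from the next entry when that wave exceeds one.
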(event EventBeginPlay
  (bind _outrownames (DataTable|GetDataTableRowNames (Variables|Default|GetDataTable)))
  (Variables|Default|SetLastIndex (- (Utilities|Array|Length _outrownames) 1))
  (for _array_element _outrownames
    (bind _returnvalue (Utilities|GetDataTableRow (Variables|Default|GetDataTable) _array_element)
      (:then
        (Utilities|Array|Add (Variables|Default|GetClassesToSpawn) (.Classtospawn (Utilities|Struct|BreakS_Spawner _returnvalue)))
        (Utilities|Array|Add (Variables|Default|GetTimeToSpawn) (.Timetospawn (Utilities|Struct|BreakS_Spawner _returnvalue)))
        (Utilities|Array|Add (Variables|Default|GetWaves) (.Wave (Utilities|Struct|BreakS_Spawner _returnvalue)))))))

(event EventTick
  (params (DeltaSeconds :type Float%20%28single-precision%29))
  (bind _currentindex (Variables|Default|GetCurrentIndex))
  (bind _waves (Variables|Default|GetWaves))
  (bind _output (Utilities|Array|Get(acopy) _waves _currentindex))
  (if (>= (Utilities|Time|GetTimeSeconds) (Utilities|Array|Get(acopy) (Variables|Default|GetTimeToSpawn) (Variables|Default|GetCurrentIndex)))
    (Utilities|FlowControl|DoOnce false :!label _label
      (:Completed
        (bind _returnvalue (Game|SpawnActorfromClass (Utilities|Array|Get(acopy) (Variables|Default|GetClassesToSpawn) (Variables|Default|GetCurrentIndex)) (Transformation|GetActorTransform) "AdjustIfPossibleButAlwaysSpawn" 0 0))
        (bind _asbp_player (Utilities|Casting|CastToBP_Player (Game|Player|GetPlayerPawn 0)))
        (Utilities|Array|AddUnique (Variables|/Game/Blueprints/Player/BP_Player.BP_Player_C|GetEnemies _asbp_player) _returnvalue)
        (Math|Integer|IncrementInt (Variables|Default|GetCurrentIndex)
          (:%20%20
            (if (> _output 1)
              (Variables|/Game/Blueprints/Player/BP_Player.BP_Player_C|SetWave _asbp_player _output)
              (goto _label Reset)
              (else
                (goto _label Reset)))))))))

(fn ConstructionScript)