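; Area-of-effect tower projectile that deals radial damage around the first spider unit it hits.
; On BeginPlay it adds every tower and tree unit in the level to an ignore list, sparing them from the blast.
; The sphere's overlap fires once, applying full, non-falloff damage centered on the spider's location, then disables the sphere's collision.
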(event OnComponentBeginOverlap(Sphere)
  (params (OverlappedComponent :type Primitive%20Component%20Object%20Reference) (OtherActor :type Actor%20Object%20Reference) (OtherComp :type Primitive%20Component%20Object%20Reference) (OtherBodyIndex :type Integer) (bFromSweep :type Boolean) (SweepResult :type Hit%20Result%20Structure%20%28by%20ref%29))
  (bind _asspider_unit (Utilities|Casting|CastToSpiderUnit OtherActor))
  (Utilities|FlowControl|DoOnce false
    (:Completed
      (Game|Damage|ApplyRadialDamage 3e+01 (Transformation|GetActorLocation _asspider_unit) 1e+02 0 (Variables|Default|GetActorsToIgnore) 0 0 true "ECC_Visibility")
      (Collision|SetCollisionEnabled (Variables|Default|GetSphere) "NoCollision"))))

(event EventBeginPlay
  (bind _outactors (Actor|GetAllActorsOfClass "/Script/GGJUA.BaseTower"))
  (for _array_element _outactors
    (Utilities|Array|AddUnique (Variables|Default|GetActorsToIgnore) _array_element))
  (bind _outactors_2 (Actor|GetAllActorsOfClass "/Script/GGJUA.TreeUnit"))
  (for _array_element_2 _outactors_2
    (Utilities|Array|AddUnique (Variables|Default|GetActorsToIgnore) _array_element_2)))

(fn ConstructionScript)