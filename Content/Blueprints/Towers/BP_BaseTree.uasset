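; Base tree tower actor with health, an HP bar widget and an empty ActivateTree function.
; On BeginPlay it binds its damage handler and passes itself to the W_TowerHPBar widget as the tower reference.
; Damage reduces CurrentHealth; at zero or below it plays a destroyed sound, spawns a fresh BP_BaseTree at its transform and destroys itself.
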(event Custom|TakeDamage
  (params (DamagedActor :type Actor%20Object%20Reference) (Damage :type Float%20%28single-precision%29) (DamageType :type Damage%20Type%20Object%20Reference) (InstigatedBy :type Controller%20Object%20Reference) (DamageCauser :type Actor%20Object%20Reference))
  (bind _output_get (Variables|Default|SetCurrentHealth (- (Variables|Default|GetCurrentHealth) Damage)))
  (if (not (> _output_get 0.0))
    (Audio|PlaySoundatLocation (Variables|Default|GetDestroyedSound) (Transformation|GetActorLocation) "0, 0, 0" 1.0 1.0 0.0 0 0 0 0)
    (Game|SpawnActorfromClass "BP_BaseTree_C" (Transformation|GetActorTransform) "Undefined" 0 0)
    (Actor|DestroyActor)))

(event EventBeginPlay
  (EventDispatchers|AssignOnTakeAnyDamage (delegate Custom|TakeDamage))
  (bind _asw_tower_hpbar (Utilities|Casting|CastToW_TowerHPBar (UserInterface|GetWidget (Variables|Default|GetHPBar))))
  (Variables|/Game/UI/W_TowerHPBar.W_TowerHPBar_C|SetTowerRef _asw_tower_hpbar self))

(fn ConstructionScript)

(fn ActivateTree)