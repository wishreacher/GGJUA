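; BP_Player is a player Blueprint that owns the HUD and tracks two resources, mana and water.
; On BeginPlay it creates the W_HUD widget, adds it to the viewport and fills both resources to their maximums.
; A looping half-second timer then adds each resource's income rate to its current value, with no clamp to the maximum.
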(event Custom|Add%20Resources
  (Variables|Resources|SetCurrentMana (+ (Variables|Resources|GetCurrentMana) (Variables|Resources|GetManaIncomeRate)))
  (Variables|Resources|SetCurrentWater (+ (Variables|Resources|GetCurrentWater) (Variables|Resources|GetWaterIncomeRate))))

(event EventBeginPlay
  (bind _returnvalue (UserInterface|CreateWidget "/Game/UI/W_HUD.W_HUD_C"))
  (bind _output_get (Variables|Resources|SetHUD _returnvalue))
  (UserInterface|Viewport|AddtoViewport _output_get 0)
  (Variables|Resources|SetCurrentMana (Variables|Resources|GetMaxMana))
  (Variables|Resources|SetCurrentWater (Variables|Resources|GetMaxWater))
  (Utilities|Time|SetTimerbyEvent (delegate Custom|Add%20Resources) 0.5 true))

(fn ConstructionScript)