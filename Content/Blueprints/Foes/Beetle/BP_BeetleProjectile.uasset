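; Projectile fired by the Beetle foe that damages built BaseTowers, TreeUnits and Ents it overlaps.
; A cast chain on the sphere's overlap picks the target type, then a per-type DoOnce applies fixed damage and disables the sphere's collision to prevent repeat hits.
; Tick prints the name of the ProjectileMovement homing target component as debug output.
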(event OnComponentBeginOverlap(Sphere)
  (params (OverlappedComponent :type Primitive%20Component%20Object%20Reference) (OtherActor :type Actor%20Object%20Reference) (OtherComp :type Primitive%20Component%20Object%20Reference) (OtherBodyIndex :type Integer) (bFromSweep :type Boolean) (SweepResult :type Hit%20Result%20Structure%20%28by%20ref%29))
  (bind _asbase_tower (Utilities|Casting|CastToBaseTower OtherActor)
    (:then
      (if (Variables|/Script/GGJUA.BaseTower|GetbIsBuilt _asbase_tower)
        (Utilities|FlowControl|DoOnce false
          (:Completed
            (Game|Damage|ApplyDamage _asbase_tower 2e+01 0 0)
            (Collision|SetCollisionEnabled (Variables|Default|GetSphere) "NoCollision")))
        (else
          (bind _astree_unit (Utilities|Casting|CastToTreeUnit OtherActor :!label _label)
            (:then
              (Utilities|FlowControl|DoOnce false
                (:Completed
                  (Game|Damage|ApplyDamage _astree_unit 2e+01 0 0)
                  (Collision|SetCollisionEnabled (Variables|Default|GetSphere) "NoCollision"))))
            (:CastFailed
              (bind _asent (Utilities|Casting|CastToEnt OtherActor))
              (Utilities|FlowControl|DoOnce false
                (:Completed
                  (Game|Damage|ApplyDamage _asent 2e+01 0 0)
                  (Collision|SetCollisionEnabled (Variables|Default|GetSphere) "NoCollision"))))))))
    (:CastFailed
      (goto _label))))

(event EventTick
  (params (DeltaSeconds :type Float%20%28single-precision%29))
  (Development|PrintString (Utilities|GetDisplayName (Variables|/Script/Engine.ProjectileMovementComponent|GetHomingTargetComponent (Variables|Default|GetProjectileMovement)))))

(fn ConstructionScript)