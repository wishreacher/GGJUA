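; BP_Beetle is a beetle foe unit with health, a configurable move speed and a health bar widget.
; On BeginPlay it stores the nearest Ent as a reference, links itself to the HP bar and sets its walk speed.
; A bound any-damage handler subtracts health and reveals the bar on non-lethal hits, or plays a death sound and destroys the actor on lethal ones.
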(event Custom|TakeDamage
  (params (DamagedActor :type Actor%20Object%20Reference) (Damage :type Float%20%28single-precision%29) (DamageType :type Damage%20Type%20Object%20Reference) (InstigatedBy :type Controller%20Object%20Reference) (DamageCauser :type Actor%20Object%20Reference))
  (bind _widget (Variables|Default|GetWidget))
  (if (> (- (Variables|Default|GetCurrentHealth) Damage) 0.0)
    (Variables|Default|SetCurrentHealth (- (Variables|Default|GetCurrentHealth) Damage))
    (if (not (Widget|IsVisible (UserInterface|GetWidget _widget)))
      (Rendering|SetVisibility _widget true false))
    (else
      (Audio|PlaySoundatLocation (Variables|Default|GetDeathSound) (Transformation|GetActorLocation) "0, 0, 0" 1.0 1.0 0.0 0 0 0 0)
      (Actor|DestroyActor))))

(event EventBeginPlay
  (EventDispatchers|BindEventtoOnTakeAnyDamage (delegate Custom|TakeDamage))
  (bind _outactors (Actor|GetAllActorsOfClass "/Script/GGJUA.Ent"))
  (bind _asent (Utilities|Casting|CastToEnt (.ReturnValue (Actor|FindNearestActor (Transformation|GetActorLocation) _outactors))))
  (Variables|Default|SetEntReference _asent)
  (bind _asw_unit_hpbar (Utilities|Casting|CastToW_UnitHPBar (UserInterface|GetWidget (Variables|Default|GetWidget))))
  (Variables|/Game/UI/W_UnitHPBar.W_UnitHPBar_C|SetUnitRef _asw_unit_hpbar self)
  (Variables|/Script/Engine.CharacterMovementComponent|SetMaxWalkSpeed (Variables|Character|GetCharacterMovement) (Variables|Default|GetMoveSpeed)))

(fn ConstructionScript)