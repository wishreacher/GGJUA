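; Melee spider enemy that damages tree units, built towers and Ents, and caches a reference to the nearest Ent on spawn.
; An attack collision, disabled at start, hits on overlap, then switches itself off and plays a sound.
; Incoming damage reveals the HP bar widget and destroys the spider at zero health.
; Stun-type damage sets a timed flag that Tick reads to switch to stunned walk speed.
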(event Custom|TakeDamage
  (params (DamagedActor :type Actor%20Object%20Reference) (Damage :type Float%20%28single-precision%29) (DamageType :type Damage%20Type%20Object%20Reference) (InstigatedBy :type Controller%20Object%20Reference) (DamageCauser :type Actor%20Object%20Reference))
  (bind _widget (Variables|Default|GetWidget))
  (if (== (Utilities|GetClass DamageType) "/Game/Blueprints/Player/DT_Stun.DT_Stun_C")
    (Variables|Default|SetbIsStunned true)
    (Utilities|Time|SetTimerbyEvent (delegate Custom|RemoveStun) 3.0))
  (if (> (- (Variables|Default|GetCurrentHealth) Damage) 0.0)
    (Variables|Default|SetCurrentHealth (- (Variables|Default|GetCurrentHealth) Damage))
    (if (not (Widget|IsVisible (UserInterface|GetWidget _widget)))
      (Rendering|SetVisibility _widget true false))
    (else
      (Audio|PlaySoundatLocation (Variables|Default|GetDeathSound) (Transformation|GetActorLocation) "0, 0, 0" 1.0 1.0 0.0 0 0 0 0)
      (Actor|DestroyActor))))

(event Custom|DealDamage
  (params (OverlappedComponent :type Primitive%20Component%20Object%20Reference) (OtherActor :type Actor%20Object%20Reference) (OtherComp :type Primitive%20Component%20Object%20Reference) (OtherBodyIndex :type Integer) (bFromSweep :type Boolean) (SweepResult :type Hit%20Result%20Structure%20%28by%20ref%29))
  (bind _astree_unit (Utilities|Casting|CastToTreeUnit OtherActor)
    (:then
      (Game|Damage|ApplyDamage _astree_unit (Variables|Default|GetDamageAmount) 0 0))
    (:CastFailed
      (bind _asbase_tower (Utilities|Casting|CastToBaseTower OtherActor)
        (:then
          (if (Variables|/Script/GGJUA.BaseTower|GetbIsBuilt _asbase_tower)
            (Game|Damage|ApplyDamage _asbase_tower (Variables|Default|GetDamageAmount) 0 0)
            (else
              (bind _asent (Utilities|Casting|CastToEnt OtherActor :!label _label))
              (Game|Damage|ApplyDamage _asent (Variables|Default|GetDamageAmount) 0 0))))
        (:CastFailed
          (goto _label)))))
  (Collision|SetCollisionEnabled (Variables|Default|GetAttackCollision) "NoCollision")
  (Audio|PlaySoundatLocation (Variables|Default|GetAttackSound) (Transformation|GetActorLocation) "0, 0, 0" 1.0 1.0 0.0 0 0 0 0))

(event Custom|RemoveStun
  (Variables|Default|SetbIsStunned false))

(event EventBeginPlay
  (EventDispatchers|BindEventtoOnTakeAnyDamage (delegate Custom|TakeDamage))
  (bind _outactors (Actor|GetAllActorsOfClass "/Script/GGJUA.Ent"))
  (bind _asent (Utilities|Casting|CastToEnt (.ReturnValue (Actor|FindNearestActor (Transformation|GetActorLocation) _outactors))))
  (Variables|Default|SetEntReference _asent)
  (bind _asw_unit_hpbar (Utilities|Casting|CastToW_UnitHPBar (UserInterface|GetWidget (Variables|Default|GetWidget))))
  (Variables|/Game/UI/W_UnitHPBar.W_UnitHPBar_C|SetUnitRef _asw_unit_hpbar self)
  (Collision|SetCollisionEnabled (Variables|Default|GetAttackCollision) "NoCollision")
  (Collision|AssignOnComponentBeginOverlap (Variables|Default|GetAttackCollision) (delegate Custom|DealDamage))
  (Variables|/Script/Engine.CharacterMovementComponent|SetMaxWalkSpeed (Variables|Character|GetCharacterMovement) (Variables|Default|GetMoveSpeed)))

(event EventTick
  (params (DeltaSeconds :type Float%20%28single-precision%29))
  (bind _charactermovement (Variables|Character|GetCharacterMovement))
  (if (Variables|Default|GetbIsStunned)
    (Variables|/Script/Engine.CharacterMovementComponent|SetMaxWalkSpeed _charactermovement (Variables|Default|GetStunnedSpeed))
    (else
      (Variables|/Script/Engine.CharacterMovementComponent|SetMaxWalkSpeed _charactermovement (Variables|Default|GetMoveSpeed)))))

(fn ConstructionScript)