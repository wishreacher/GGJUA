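; BP_Ent is an Ent character whose death loses the game.
; On BeginPlay it binds to its any-damage event, and each hit subtracts from its current health.
; While health remains it plays a hit montage; otherwise it pauses the game, shows the lose screen widget, switches input to UI only and plays the lose sound.
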(event Custom|TakeDamage
  (params (DamagedActor :type Actor%20Object%20Reference) (Damage :type Float%20%28single-precision%29) (DamageType :type Damage%20Type%20Object%20Reference) (InstigatedBy :type Controller%20Object%20Reference) (DamageCauser :type Actor%20Object%20Reference))
  (bind _output_get (Variables|Default|SetCurrentHealth (- (Variables|Default|GetCurrentHealth) Damage)))
  (if (> _output_get 0.0)
    (Animation|PlayAnimMontage "/Game/Blueprints/Ent/Animations/AM_Hit.AM_Hit" 1.0 "None")
    (else
      (Game|SetGamePaused true)
      (bind _returnvalue (UserInterface|CreateWidget "/Game/UI/W_LoseScreen.W_LoseScreen_C"))
      (UserInterface|Viewport|AddtoViewport _returnvalue 0)
      (Input|SetInputModeUIOnly 0 0 "DoNotLock" false)
      (Audio|PlaySound2D "/Game/SFX/Lose.Lose" 1.0 1.0 0.0 0 0))))

(event EventBeginPlay
  (EventDispatchers|AssignOnTakeAnyDamage (delegate Custom|TakeDamage)))

(fn ConstructionScript)