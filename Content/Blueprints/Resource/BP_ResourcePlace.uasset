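; BP_ResourcePlace is a capturable resource spot that boosts the player's water and mana income once built.
; AttemptToActivateSpot deducts water and mana costs, starts a build timer and shows an altar build-bar widget, or displays a not-enough-resources widget.
; ActivateSpot raises income rates, plays a capture sound and montage, swaps the mesh material and hides the bar.
; PendingActivation and IsActive flags block repeat purchases.
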(fn ConstructionScript)

(fn AttempttoActivateSpot
  (bind _widget (Variables|Default|GetWidget))
  (if (not (Variables|Default|GetPendingActivation))
    (if (not (Variables|Default|GetIsActive))
      (bind _asbp_player (Utilities|Casting|CastToBP_Player (Game|Player|GetPlayerPawn 0)))
      (bind _output_get (Variables|Default|SetAs%20BP%20Player _asbp_player))
      (if (and (>= (- (Variables|/Game/Blueprints/Player/BP_Player.BP_Player_C|GetCurrentMana _asbp_player) (Variables|Default|GetManaCost)) 0.0) (>= (- (Variables|/Game/Blueprints/Player/BP_Player.BP_Player_C|GetCurrentWater _asbp_player) (Variables|Default|GetWaterCost)) 0.0))
        (Variables|/Game/Blueprints/Player/BP_Player.BP_Player_C|SetCurrentWater _output_get (- (Variables|/Game/Blueprints/Player/BP_Player.BP_Player_C|GetCurrentWater _output_get) (Variables|Default|GetWaterCost)))
        (Variables|/Game/Blueprints/Player/BP_Player.BP_Player_C|SetCurrentMana _output_get (- (Variables|/Game/Blueprints/Player/BP_Player.BP_Player_C|GetCurrentMana _output_get) (Variables|Default|GetManaCost)))
        (bind _returnvalue (Utilities|Time|SetTimerbyEvent (EventDispatchers|CreateEvent :!event ActivateSpot) (Variables|Default|GetTimeToBuild)))
        (Variables|Default|SetPendingActivation true)
        (Variables|Default|SetTimeToVBuildTimerHandle _returnvalue)
        (Rendering|SetVisibility _widget true false)
        (bind _asw_altar_build_bar (Utilities|Casting|CastToW_AltarBuildBar (UserInterface|GetWidget _widget)))
        (Variables|/Game/UI/W_AltarBuildBar.W_AltarBuildBar_C|SetAltarRef _asw_altar_build_bar self)
        (else
          (Utilities|IsValid (LocalVariables|GetWidgetWidget)
            (:Is%20Not%20Valid
              (bind _returnvalue_2 (UserInterface|CreateWidget "/Game/UI/W_NotEnoughResources.W_NotEnoughResources_C"))
              (LocalVariables|SetWidgetWidget _returnvalue_2)
              (UserInterface|Viewport|AddtoViewport _returnvalue_2 0))))))))

(fn ActivateSpot
  (bind _as_bp_player (Variables|Default|GetAs%20BP%20Player))
  (Variables|/Game/Blueprints/Player/BP_Player.BP_Player_C|SetWaterIncomeRate _as_bp_player (+ (Variables|/Game/Blueprints/Player/BP_Player.BP_Player_C|GetWaterIncomeRate _as_bp_player) (Variables|Default|GetWaterPerSecond)))
  (Variables|/Game/Blueprints/Player/BP_Player.BP_Player_C|SetManaIncomeRate _as_bp_player (+ (Variables|/Game/Blueprints/Player/BP_Player.BP_Player_C|GetManaIncomeRate _as_bp_player) (Variables|Default|GetManaPerSecond)))
  (Variables|Default|SetIsActive true)
  (Audio|PlaySoundatLocation "/Game/SFX/capture_of_resources.capture_of_resources" (Transformation|GetActorLocation _as_bp_player) "0, 0, 0" 1.0 1.0 0.0 0 0 0 0)
  (Animation|Montage|MontagePlay (Components|SkeletalMesh|GetAnimInstance (Variables|Default|GetSkeletalMesh)) (Variables|Default|GetActivationMontage) 1.0 "MontageLength" 0.0 true)
  (Rendering|Material|SetMaterial (Variables|Default|GetSkeletalMesh) 0 (Variables|Default|GetActivatedMaterial))
  (Utilities|Time|ClearandInvalidateTimerbyHandle (Variables|Default|GetTimeToVBuildTimerHandle))
  (Rendering|SetVisibility (Variables|Default|GetWidget) false false))