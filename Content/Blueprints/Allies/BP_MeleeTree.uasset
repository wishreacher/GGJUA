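; BP_MeleeTree is an allied actor with health that is destroyed when damage depletes it.
; On BeginPlay it binds its damage handler, which subtracts each non-lethal hit from CurrentHealth and calls DestroyActor on a lethal one.
; While its widget is hidden, a surviving hit sets the actor as the W_HPBar's UnitRef and shows the health bar.
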(event Custom|TakeDamage
  (params (DamagedActor :type Actor%20Object%20Reference) (Damage :type Float%20%28single-precision%29) (DamageType :type Damage%20Type%20Object%20Reference) (InstigatedBy :type Controller%20Object%20Reference) (DamageCauser :type Actor%20Object%20Reference))
  (bind _widget (Variables|Default|GetWidget))
  (bind _returnvalue (UserInterface|GetWidget _widget))
  (if (> (- (Variables|Default|GetCurrentHealth) Damage) 0.0)
    (Variables|Default|SetCurrentHealth (- (Variables|Default|GetCurrentHealth) Damage))
    (if (not (Widget|IsVisible _returnvalue))
      (bind _asw_hpbar (Utilities|Casting|CastToW_HPBar _returnvalue))
      (Variables|/Game/UI/W_HPBar.W_HPBar_C|SetUnitRef _asw_hpbar self)
      (Widget|SetVisibility _returnvalue "Visible"))
    (else
      (Actor|DestroyActor))))

(event EventBeginPlay
  (EventDispatchers|BindEventtoOnTakeAnyDamage (delegate Custom|TakeDamage)))

(fn ConstructionScript)