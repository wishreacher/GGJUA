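; BP_Hammer is an allied melee unit that damages SpiderUnit enemies with its two arms.
; Arm collision starts disabled; an overlap with a spider applies damage, plays the attack sound and disables both arms again, with re-enabling handled outside this graph.
; Incoming damage lowers health, plays a hit montage, then requests a hit sound and shows the linked HP bar widget, or destroys the actor when lethal.
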(event Custom|TakeDamage
  (params (DamagedActor :type Actor%20Object%20Reference) (Damage :type Float%20%28single-precision%29) (DamageType :type Damage%20Type%20Object%20Reference) (InstigatedBy :type Controller%20Object%20Reference) (DamageCauser :type Actor%20Object%20Reference))
  (if (> (- (Variables|Default|GetCurrentHealth) Damage) 0.0)
    (Variables|Default|SetCurrentHealth (- (Variables|Default|GetCurrentHealth) Damage))
    (Animation|Montage|PlayMontage 0 (Variables|Default|GetHitMontage)
      (:then
        (Audio|PlaySoundatLocation (Variables|Default|GetHitSound) (Transformation|GetActorLocation) "0, 0, 0" 1.0 1.0 0.0 0 0 0 0)
        (Rendering|SetVisibility (Variables|Default|GetWidget) true false)))
    (else
      (Actor|DestroyActor))))

(event Custom|DealDamage
  (params (OverlappedComponent :type Primitive%20Component%20Object%20Reference) (OtherActor :type Actor%20Object%20Reference) (OtherComp :type Primitive%20Component%20Object%20Reference) (OtherBodyIndex :type Integer) (bFromSweep :type Boolean) (SweepResult :type Hit%20Result%20Structure%20%28by%20ref%29))
  (bind _asspider_unit (Utilities|Casting|CastToSpiderUnit OtherActor))
  (Game|Damage|ApplyDamage _asspider_unit (Variables|Default|GetDamageAmount) 0 0)
  (Collision|SetCollisionEnabled (Variables|Default|GetLeftArm) "NoCollision")
  (Collision|SetCollisionEnabled (Variables|Default|GetRightArm) "NoCollision")
  (Audio|PlaySoundatLocation (Variables|Default|GetAttackSound) (Transformation|GetActorLocation) "0, 0, 0" 1.0 1.0 0.0 0 0 0 0))

(event EventBeginPlay
  (EventDispatchers|BindEventtoOnTakeAnyDamage (delegate Custom|TakeDamage))
  (Collision|SetCollisionEnabled (Variables|Default|GetRightArm) "NoCollision")
  (Collision|SetCollisionEnabled (Variables|Default|GetLeftArm) "NoCollision")
  (Collision|AssignOnComponentBeginOverlap (Variables|Default|GetLeftArm) (delegate Custom|DealDamage))
  (Collision|AssignOnComponentBeginOverlap (Variables|Default|GetRightArm) (delegate Custom|DealDamage))
  (Variables|/Script/Engine.CharacterMovementComponent|SetMaxWalkSpeed (Variables|Character|GetCharacterMovement) (Variables|Default|GetMoveSpeed))
  (bind _asw_unit_hpbar (Utilities|Casting|CastToW_UnitHPBar (UserInterface|GetWidget (Variables|Default|GetWidget))))
  (Variables|/Game/UI/W_UnitHPBar.W_UnitHPBar_C|SetUnitRef _asw_unit_hpbar self))

(fn ConstructionScript)